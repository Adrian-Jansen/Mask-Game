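; Child weapon Blueprint, apparently of BP_WeaponBase, that implements Fire by launching a projectile from the player.
; Fire reads the player's location through the combat component reference and spawns BP_ProjectileBase at a fixed height above it, passing in the weapon's damage.
; The spawn sets only a location, with no aim rotation.
; BeginPlay is disabled and the construction script only calls the parent.
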(event `self.Fire`
  (bind (_returnvalue_x _returnvalue_y _returnvalue_z) (`KismetMathLibrary.BreakVector` (`self.K2_GetActorLocation` (`/Game/ThirdPerson/Blueprints/BPC_Combat.PlayerRef` (`self.CombatComponentRef`)))))
  (`|SpawnActorFromClass` "/Game/Weapons/BP_ProjectileBase.BP_ProjectileBase_C" (`KismetMathLibrary.MakeTransform` (`KismetMathLibrary.MakeVector` _returnvalue_x _returnvalue_y (+ _returnvalue_z 150.0))) "Undefined" "MultiplyWithRoot" null (`self.Get Damage`) null))

(fn `UserConstructionScript`
  (`parent.UserConstructionScript`))