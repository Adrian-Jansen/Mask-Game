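; Base weapon Blueprint that fires automatically on a looping timer, leaving the Fire event empty.
; BeginPlay starts the timer, using GetFireRate once as the interval in seconds, so later modifier changes do not retime it.
; Getters scale fire rate and bullet speed by modifiers from CombatComponentRef and take projectile count straight from that component, while damage is returned unmodified.
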(event `self.ReceiveBeginPlay`
  (`KismetSystemLibrary.K2_SetTimerDelegate` (delegate `Fire`) (`self.Get Fire Rate`) true true))

(event `Fire`)

(fn `Get Bullet Speed`
  (returns (Value :type "Float (double-precision)"))
  (return (* (`self.Bullet Speed`) (`/Game/ThirdPerson/Blueprints/BPC_Combat.Bullet Speed Modifier` (`self.CombatComponentRef`)))))

(fn `Get Damage`
  (returns (Value :type "Float (double-precision)"))
  (return (`self.Damage`)))

(fn `Get Fire Rate`
  (returns (ReturnValue :type "Float (double-precision)"))
  (return (* (`self.FireRate`) (`/Game/ThirdPerson/Blueprints/BPC_Combat.Fire Rate Modifier` (`self.CombatComponentRef`)))))

(fn `Get Projectile Count`
  (returns (Value :type "Float (double-precision)"))
  (return (`/Game/ThirdPerson/Blueprints/BPC_Combat.Projectile Count` (`self.CombatComponentRef`))))

(fn `UserConstructionScript`)