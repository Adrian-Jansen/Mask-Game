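; Base projectile Blueprint for weapons that damages actors with a health component and can penetrate them.
; On BeginPlay its collision ignores the instigator and ProjectileMovement launches it along local X at BulletSpeed.
; Each overlap with a BPC_HealthSystem owner applies Damage and decrements BulletPenetration, destroying the projectile once that runs out.
; The Hit event is empty, and older hit-damage and Niagara impact-effect nodes are left disconnected.
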(event `self.ReceiveBeginPlay`
  (`PrimitiveComponent.IgnoreActorWhenMoving` (`self.Collision`) (`self.GetInstigator`) true)
  (`ProjectileMovementComponent.SetVelocityInLocalSpace` (`self.ProjectileMovement`) (`KismetMathLibrary.MakeVector` (`self.Bullet Speed`))))

(event `self.ReceiveHit`
  (params (MyComp :type "PrimitiveComponent Object Reference") (Other :type "Actor Object Reference") (OtherComp :type "PrimitiveComponent Object Reference") (bSelfMoved :type Boolean) (HitLocation :type "Vector Structure") (HitNormal :type "Vector Structure") (NormalImpulse :type "Vector Structure") (Hit :type "HitResult Structure (by ref)")))

(event `self.Collision.OnComponentBeginOverlap`
  (params (OverlappedComponent :type "PrimitiveComponent Object Reference") (OtherActor :type "Actor Object Reference") (OtherComp :type "PrimitiveComponent Object Reference") (OtherBodyIndex :type Integer) (bFromSweep :type Boolean) (SweepResult :type "HitResult Structure (by ref)"))
  (bind _returnvalue (`self.GetComponentByClass` OtherActor "/Game/ThirdPerson/Blueprints/BPC_HealthSystem.BPC_HealthSystem_C"))
  (`/Engine/EditorBlueprintResources/StandardMacros.IsValid` _returnvalue
    (:`Is Valid`
      (`/Game/ThirdPerson/Blueprints/BPC_HealthSystem.Decrease Health` _returnvalue (`self.Damage`))
      (bind _result (`/Engine/EditorBlueprintResources/StandardMacros.DecrementFloat` (`self.Bullet Penetration`))
        (:`  `
          (if (<= _result 0.0)
            (`self.K2_DestroyActor`)))))))

(fn `UserConstructionScript`)