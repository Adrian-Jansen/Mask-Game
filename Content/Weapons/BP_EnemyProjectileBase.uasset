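; BP_EnemyProjectileBase is a base enemy projectile that damages actors it overlaps.
; On BeginPlay its collision ignores the instigator while moving, and ProjectileMovement launches it along local X at BulletSpeed.
; An overlap with an actor that has a BPC_HealthSystem component applies Damage through that component and destroys the projectile; other overlaps are ignored.
; A Niagara impact effect exists in the graph but is disconnected.
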(event `self.ReceiveBeginPlay`
  (`PrimitiveComponent.IgnoreActorWhenMoving` (`self.Collision`) (`self.GetInstigator`) true)
  (`ProjectileMovementComponent.SetVelocityInLocalSpace` (`self.ProjectileMovement`) (`KismetMathLibrary.MakeVector` (`self.Bullet Speed`))))

(event `self.Collision.OnComponentBeginOverlap`
  (params (OverlappedComponent :type "PrimitiveComponent Object Reference") (OtherActor :type "Actor Object Reference") (OtherComp :type "PrimitiveComponent Object Reference") (OtherBodyIndex :type Integer) (bFromSweep :type Boolean) (SweepResult :type "HitResult Structure (by ref)"))
  (bind _returnvalue (`self.GetComponentByClass` OtherActor "/Game/ThirdPerson/Blueprints/BPC_HealthSystem.BPC_HealthSystem_C"))
  (`/Engine/EditorBlueprintResources/StandardMacros.IsValid` _returnvalue
    (:`Is Valid`
      (`/Game/ThirdPerson/Blueprints/BPC_HealthSystem.Apply Damage` _returnvalue (`self.Damage`))
      (`self.K2_DestroyActor`))))

(fn `UserConstructionScript`)