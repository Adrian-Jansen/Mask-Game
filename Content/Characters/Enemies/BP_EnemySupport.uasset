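; Support enemy that periodically fires a fan of projectiles when the player is nearby.
; A looping timer started on BeginPlay checks the distance to the player and, when in range, plays a 2D sound and calls FireCone.
; FireCone spawns BulletCount enemy projectiles spread evenly across ConeAngle, centred on the actor's yaw, with fixed damage, speed and penetration.
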(event `self.ReceiveBeginPlay`
  (`KismetSystemLibrary.K2_SetTimerDelegate` (delegate `Shoot`) 2.0 true))

(event `Shoot`
  (if (< (`self.GetDistanceTo` (`GameplayStatics.GetPlayerCharacter` 0)) 750.0)
    (`GameplayStatics.PlaySound2D` "/Game/Audio/enemy_bulletsupport.enemy_bulletsupport" 1.0 1.0 0.0 null null)
    (`self.FireCone`)))

(fn `FireCone`
  (locals (BulletCount :type Integer :default 3) (ConeAngle :type "Float (double-precision)" :default 40.0))
  (bind (_returnvalue_roll _returnvalue_pitch _returnvalue_yaw) (`KismetMathLibrary.BreakRotator` (`self.K2_GetActorRotation`)))
  (for _index (range (`local.BulletCount`))
    (`|SpawnActorFromClass` "/Game/Weapons/BP_EnemyProjectileBase.BP_EnemyProjectileBase_C" (`KismetMathLibrary.MakeTransform` (`self.K2_GetActorLocation`) (`KismetMathLibrary.MakeRotator` 0.0 0.0 (- (+ (* _index (/ (`local.ConeAngle`) (- (`local.BulletCount`) 1))) _returnvalue_yaw) (/ (`local.ConeAngle`) 2.0)))) "AlwaysSpawn" "MultiplyWithRoot" null 5.0 450.0 1.0 null)))

(fn `UserConstructionScript`
  (`parent.UserConstructionScript`))