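; Base enemy actor that chases the player and deals contact damage until it is killed.
; Tick reissues AIMoveTo toward the player, while overlap applies damage immediately and starts a looping timer for repeat hits, cleared when overlap ends.
; On the health component's Death event, it increments the HUD score, plays a sound, destroys itself and spawns an experience shard, plus a rare random power-up from a data asset.
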(event `self.ReceiveTick`
  (params (DeltaSeconds :type "Float (single-precision)"))
  (`|AIMoveTo` self (0.0 0.0 0.0) (`GameplayStatics.GetPlayerCharacter` 0) 0.0))

(event `self.ReceiveActorBeginOverlap`
  (params (OtherActor :type "Actor Object Reference"))
  ; Damage On Overlap with player
  (if (== OtherActor (`GameplayStatics.GetPlayerCharacter` 0))
    (`/Game/ThirdPerson/Blueprints/BPC_HealthSystem.Decrease Health` (`self.GetComponentByClass` OtherActor "/Game/ThirdPerson/Blueprints/BPC_HealthSystem.BPC_HealthSystem_C") 10.0)
    (bind _returnvalue (`KismetSystemLibrary.K2_SetTimerDelegate` (delegate `Damage`) 1.0 true))
    (set `self.Damage Timer` _returnvalue)))

(event `Damage`
  ; Damage On Overlap with player
  (bind _returnvalue (`self.GetComponentByClass` (stale `self.ReceiveActorBeginOverlap` OtherActor) "/Game/ThirdPerson/Blueprints/BPC_HealthSystem.BPC_HealthSystem_C"))
  (`/Engine/EditorBlueprintResources/StandardMacros.IsValid` _returnvalue
    (:`Is Valid`
      (`/Game/ThirdPerson/Blueprints/BPC_HealthSystem.Decrease Health` _returnvalue 10.0))))

(event `self.ReceiveActorEndOverlap`
  (params (OtherActor :type "Actor Object Reference"))
  ; Damage On Overlap with player
  (if (== OtherActor (`GameplayStatics.GetPlayerCharacter` 0))
    (`KismetSystemLibrary.K2_ClearAndInvalidateTimerHandle` (`self.Damage Timer`))))

(event `self.BPC_HealthSystem.Death`
  (`/Engine/EditorBlueprintResources/StandardMacros.IncrementInt` (`/Game/ThirdPerson/UI/WB_Score.CurrentScore` (`/Game/ThirdPerson/UI/WB_HUD.WB_Score` (`/Game/ThirdPerson/Blueprints/BPC_UISystem.HudRef` (`self.GetComponentByClass` (`GameplayStatics.GetPlayerCharacter` 0) "/Game/ThirdPerson/Blueprints/BPC_UISystem.BPC_UISystem_C"))))
    (:`  `
      (`GameplayStatics.PlaySound2D` "/Game/Audio/enemy_death.enemy_death" 1.0 1.0 0.0 null null)
      (`self.K2_DestroyActor`)
      (`|SpawnActorFromClass` "/Game/Powerups/BP_ExpShard.BP_ExpShard_C" (`KismetMathLibrary.MakeTransform` (`self.K2_GetActorLocation`) (`KismetMathLibrary.RandomRotator` false)) "AlwaysSpawn" "MultiplyWithRoot" null null)
      (if (< (`KismetMathLibrary.RandomFloatInRange` 0.0 100.0) 5.0)
        (`|SpawnActorFromClass` (`KismetArrayLibrary.Array_Random` (`/Game/Powerups/BPDA_PowerUps.PowerUps` (`self.DA_PowerUpsDrop`))) (`KismetMathLibrary.MakeTransform` (`self.K2_GetActorLocation`)) "AlwaysSpawn" "MultiplyWithRoot" null null)))))

(fn `UserConstructionScript`)