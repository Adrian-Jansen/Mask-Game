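; Enemy spawner that continuously spawns random enemy types on the navmesh in a ring around the player, with difficulty rising over time.
; Looping timers shorten the spawn interval and lower the powerup drop rate, while one-shot timers add ranged, then support enemies to the pool.
; Each rate change re-arms the spawn timer.
; Each spawn receives the current drop rate, plus health and walk speed bonuses scaled by elapsed game time.
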(event `SetNewSpawnRate`
  (set `self.SpawnRate` (`KismetMathLibrary.FClamp` (/ (`self.SpawnRate`) 1.1) 0.01 5.0))
  (`self.UpdateSpawnRate`))

(event `SpawnRangedEnemies`
  (`KismetArrayLibrary.Array_Add` (`self.EnemyTypes`) "/Game/Characters/Enemies/BP_EnemyRanged.BP_EnemyRanged_C"))

(event `Spawn Support`
  (`KismetArrayLibrary.Array_Add` (`self.EnemyTypes`) "/Game/Characters/Enemies/BP_EnemySupport.BP_EnemySupport_C"))

(event `Update Drop Rate`
  (set `self.EnemyPowerupDropRate` (`KismetMathLibrary.FClamp` (- (`self.EnemyPowerupDropRate`) 0.1) 0.5 100.0)))

(event `self.ReceiveBeginPlay`
  (`|ExecutionSequence`
    (:`then_0`
      (`KismetSystemLibrary.K2_SetTimerDelegate` (delegate `SetNewSpawnRate`) 10.0 true)
      (`KismetSystemLibrary.K2_SetTimerDelegate` (delegate `SpawnRangedEnemies`) 60.0)
      (`KismetSystemLibrary.K2_SetTimerDelegate` (delegate `Spawn Support`) 180.0)
      (`KismetSystemLibrary.K2_SetTimerDelegate` (delegate `Update Drop Rate`) 30.0 true))
    (:`then_1`
      (`KismetSystemLibrary.K2_SetTimerDelegate` (delegate `Spawn Enemy`) (`self.SpawnRate`) true false -1.0 :!label _label))))

(event `UpdateSpawnRate`
  (goto _label))

(event `Spawn Enemy`
  (bind _returnvalue (`|SpawnActorFromClass` (`KismetArrayLibrary.Array_Random` (`self.EnemyTypes`)) (`KismetMathLibrary.MakeTransform` (`NavigationSystemV1.K2_ProjectPointToNavigation` (+ (* (`KismetMathLibrary.Normal` (`KismetMathLibrary.MakeVector` (.x (`KismetMathLibrary.RandomUnitVector`)) (.y (`KismetMathLibrary.RandomUnitVector`)))) (`KismetMathLibrary.RandomFloatInRange` 2000.0 4000.0)) (`self.K2_GetActorLocation` (`GameplayStatics.GetPlayerCharacter` 0))))) "Undefined" "MultiplyWithRoot" null (`self.EnemyPowerupDropRate`) null))
  (`/Engine/EditorBlueprintResources/StandardMacros.IsValid` _returnvalue
    (:`Is Valid`
      (bind _bpc_healthsystem (`/Game/Characters/Enemies/BP_EnemyBase.BPC_HealthSystem` _returnvalue))
      (bind _output_get (set `/Game/ThirdPerson/Blueprints/BPC_HealthSystem.Max Health` (+ (`/Game/ThirdPerson/Blueprints/BPC_HealthSystem.Max Health` _bpc_healthsystem) (/ (`KismetMathLibrary.FFloor` (`KismetSystemLibrary.GetGameTimeInSeconds`)) 5)) _bpc_healthsystem))
      (`/Game/ThirdPerson/Blueprints/BPC_HealthSystem.Set Health` _bpc_healthsystem _output_get)
      (bind _charactermovement (`Character.CharacterMovement` _returnvalue))
      (set `CharacterMovementComponent.MaxWalkSpeed` (+ (`CharacterMovementComponent.MaxWalkSpeed` _charactermovement) (/ (`KismetMathLibrary.FFloor` (`KismetSystemLibrary.GetGameTimeInSeconds`)) 4)) _charactermovement))))

(fn `UserConstructionScript`)